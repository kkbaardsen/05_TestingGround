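; AI controller for patrolling guard NPCs that runs the guard behavior tree on its blackboard from BeginPlay.
; AI perception stores sensed actors lacking the "Enemy" tag in the enemy blackboard key, clearing it when sensing fails.
; Tick sets the guard pawn's Aiming flag whenever a valid focus actor exists.
; A helper function writes the guard's first patrol point to the Waypoint key.
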(event OnTargetPerceptionUpdated(AIPerception)
  (params (Actor :type Actor%20Object%20Reference) (Stimulus :type AI%20Stimulus%20Structure))
  (bind _enemykey (Variables|Default|GetEnemyKey))
  (bind _blackboardcomp (Variables|Default|GetBlackboardComp))
  ;[1 1 1] AI Perception PrintToScreen
  (if (not (Actor|ActorHasTag Actor "Enemy"))
    (if (.bSuccessfullySensed (Utilities|Struct|BreakAIStimulus Stimulus))
      (AI|Components|Blackboard|SetValueasObject _blackboardcomp _enemykey Actor)
      (else
        (AI|Components|Blackboard|ClearValue _blackboardcomp _enemykey)))))

(event EventBeginPlay
  ;[1 1 1] Blackboard Behaviour Tree
  (bind _blackboardcomponent (Class|AIController|UseBlackboard "/Game/1_Blueprints/NPC_AI/Behaviour/BB_Patrol_Data.BB_Patrol_Data"))
  (Variables|Default|SetBlackboardComp _blackboardcomponent)
  (AI|RunBehaviorTree "/Game/1_Blueprints/NPC_AI/Behaviour/BT_GuardBehaviour.BT_GuardBehaviour"))

(event EventTick
  (params (DeltaSeconds :type Float%20%28single-precision%29))
  ;[1 1 1] Aiming
  (bind _asbp_patrolling_guard (Utilities|Casting|CastToBP_PatrollingGuard (Pawn|GetControlledPawn)))
  (Variables|/Game/1_Blueprints/NPC_AI/BP_PatrollingGuard.BP_PatrollingGuard_C|SetAiming _asbp_patrolling_guard (Utilities|IsValid (Class|AIController|GetFocusActor))))

(fn ConstructionScript)

(fn FindPatrolRoute
  (params (Blackboard :type Blackboard%20Component%20Object%20Reference))
  (bind _asbp_patrolling_guard (Utilities|Casting|CastToBP_PatrollingGuard (Pawn|GetControlledPawn)))
  (AI|Components|Blackboard|SetValueasObject Blackboard (Utilities|Name|MakeLiteralName "Waypoint") (Utilities|Array|Get(acopy) (Variables|/Game/1_Blueprints/NPC_AI/BP_PatrollingGuard.BP_PatrollingGuard_C|GetPatrol%20Points _asbp_patrolling_guard))))